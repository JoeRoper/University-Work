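; Blueprint function library of bullet impact helpers, apparently supporting surface penetration.
; SpawnBulletHole attaches a short-lived decal to the hit component, aligned to the impact normal.
; GetSurfaceDensity maps surface types such as plaster, wood and concrete to density values.
; LineTraceExitLocation finds an actor's far-side exit by tracing backward from beyond its bounds, ignoring and re-tracing past other actors until it hits the target.
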(fn SpawnBulletHole
  (params (Hit :type Hit%20Result%20Structure))
  (bind _returnvalue (Class|GameplayStatics|SpawnDecalAttached "/Game/Media/M_BulletHoleDecal.M_BulletHoleDecal" "1.000000,10.000000,10.000000" (.hitcomponent Hit) "None" (.location Hit) (Math|Conversions|RotationFromXVector (.impactnormal Hit)) "KeepWorldPosition" 1e+01))
  (Rendering|Components|Decal|SetFadeScreenSize _returnvalue 0.001))

(fn GetSurfaceDensity
  (params (Surface :type EPhysicalSurface%20Enum :default "SurfaceType_Default"))
  (return (Utilities|Select :Index Surface :SurfaceType_Default 1.0 :SurfaceType1 0.15 :SurfaceType2 0.25 :SurfaceType3 0.5)))

(fn LineTraceExitLocation
  (params (EntryLocation :type Vector) (Direction :type Vector) (Actor :type Actor%20Object%20Reference))
  (bind _boxextent (Collision|GetActorBounds Actor true true))
  (LocalVariables|SetTraceDistance (* (Math|Float|Max(Float) (.x _boxextent) (.y _boxextent) (.z _boxextent)) 4.0))
  (bind _output_get (LocalVariables|SetTraceStart (+ EntryLocation (* Direction (LocalVariables|GetTraceDistance)))))
  (LocalVariables|SetTraceEnd (+ _output_get (* Direction (* (LocalVariables|GetTraceDistance) -1.0))))
  (bind (_outhit _returnvalue) (Collision|LineTraceByChannel 0 (LocalVariables|GetTraceStart) (LocalVariables|GetTraceEnd) "TraceTypeQuery1" false (LocalVariables|GetIgnore%20List) "None" :!label _label))
  (if _returnvalue
    (if (!= (.HitActor (Collision|BreakHitResult _outhit)) Actor)
      (Utilities|Array|Add (LocalVariables|GetIgnore%20List) (.HitActor (Collision|BreakHitResult _outhit)))
      (LocalVariables|SetTraceStart (.ImpactPoint (Collision|BreakHitResult _outhit)))
      (goto _label)
      (else
        (return true _outhit)))
    (else
      (return false ""))))